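; Collectible pickup actor whose cylinder moves vertically on a timeline, replaying after a short delay.
; When the player overlaps it, it caches location, scale and light intensity, then one collection timeline lerps it toward the player while shrinking it and dimming its point light.
; On finish it calls DestroyActor, then increments the grabbed count in F4LGameInstance and changes the score by AddScore.
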(event EventBeginPlay
  (bind _moveupdown (Timeline|CollectibleUpDownMove PlayFromStart)
    (:Update
      (Transformation|SetRelativeLocation (Variables|Default|GetCylinder) (Math|Vector|MakeVector 0.0 0.0 _moveupdown) false false))
    (:MoveDone
      (Utilities|FlowControl|Delay 2.0)
      (Timeline|CollectibleUpDownMove PlayFromStart))))

(event Collision|EventActorBeginOverlap
  (params (OtherActor :type Actor%20Object%20Reference))
  (Utilities|IsPlayer OtherActor
    (:IsPlayer
      (CallFunction|SetStartingValues)
      (bind (_direction _collectionprogress _scaletime _shine) (Timeline|CollectionTimeline Play)
        (:Update
          (CallFunction|MovetoPlayer _collectionprogress)
          (CallFunction|ScaleShape _scaletime)
          (CallFunction|LightBrightness _shine))
        (:Finished
          (Actor|DestroyActor)
          (CallFunction|GetCollectiblesNumber)
          (Utilities|ChangeScore (Variables|Default|GetaddScore)))))))

(event EventTick
  (params (DeltaSeconds :type Float%20%28single-precision%29)))

(fn ConstructionScript)

(fn SetStartingValues
  (Variables|Default|SetLerpStart (Transformation|GetActorLocation))
  (Variables|Default|SetScale (Transformation|GetActorScale3D))
  (Variables|Default|SetIntensity (Variables|/Script/Engine.LightComponentBase|GetIntensity (Variables|Default|GetPointLight))))

(fn MovetoPlayer
  (params (Alpha :type Float%20%28single-precision%29))
  (Transformation|SetActorLocation (Math|Vector|Lerp(Vector) (Variables|Default|GetLerpStart) (Transformation|GetActorLocation (Game|Player|GetPlayerPawn 0)) Alpha) false false))

(fn ScaleShape
  (params (Alpha :type Float%20%28single-precision%29))
  (Transformation|SetActorScale3D (Math|Vector|Lerp(Vector) (Variables|Default|GetScale) "0, 0, 0" Alpha)))

(fn LightBrightness
  (params (Alpha :type Float%20%28single-precision%29))
  (Rendering|Components|Light|SetIntensity (Variables|Default|GetPointLight) (Math|Float|Lerp (Variables|Default|GetIntensity) 0.0 Alpha)))

(fn GetCollectiblesNumber
  (bind _asf4lgame_instance (Utilities|Casting|CastToF4LGameInstance (Game|GetGameInstance)))
  (Variables|/Game/GameInstances/F4LGameInstance.F4LGameInstance_C|SetgrabbedCollectibles _asf4lgame_instance (+ (Variables|/Game/GameInstances/F4LGameInstance.F4LGameInstance_C|GetgrabbedCollectibles _asf4lgame_instance) 1)))