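; Thunder projectile that damages whatever actor it hits and flashes a light on impact.
; On Hit, the ThunderSplash timeline drives the PointLight intensity, and its Update pin also leads through a short delay to DestroyActor.
; If the player pawn was hit, an orange-red camera fade in and back out is chained after DestroyActor, with another delay between the two fades.
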(event Collision|EventActorBeginOverlap
  (params (OtherActor :type Actor%20Object%20Reference)))

(event EventTick
  (params (DeltaSeconds :type Float%20%28single-precision%29)))

(event Collision|EventHit
  (params (MyComp :type Primitive%20Component%20Object%20Reference) (Other :type Actor%20Object%20Reference) (OtherComp :type Primitive%20Component%20Object%20Reference) (bSelfMoved :type Boolean) (HitLocation :type Vector :default "0, 0, 0") (HitNormal :type Vector :default "0, 0, 0") (NormalImpulse :type Vector :default "0, 0, 0") (Hit :type Hit%20Result%20Structure%20%28by%20ref%29))
  (Game|Damage|ApplyDamage Other 1.0 0 0)
  (bind _lightintensity (Timeline|thunderSplash PlayFromStart)
    (:Update
      (Rendering|Components|Light|SetIntensity (Variables|Default|GetPointLight) _lightintensity)
      (Utilities|FlowControl|Delay 0.2)
      (Actor|DestroyActor)
      (if (== Other (Game|Player|GetPlayerPawn 0))
        (CameraFades|StartCameraFade (Game|GetPlayerCameraManager 0) 0.0 1.0 0.4 "(R=1.000000,G=0.071799,B=0.000000,A=1.000000)" false false)
        (Utilities|FlowControl|Delay 0.4)
        (CameraFades|StartCameraFade (Game|GetPlayerCameraManager 0) 1.0 0.0 0.4 "(R=1.000000,G=0.071799,B=0.000000,A=1.000000)" false false)))))

(fn ConstructionScript)