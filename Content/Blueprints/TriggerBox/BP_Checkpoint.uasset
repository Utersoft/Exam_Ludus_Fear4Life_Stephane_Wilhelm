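; BP_Checkpoint is a one-use checkpoint actor that updates the player's respawn position when touched.
; A timeline bobs its Box component along Z, restarting two seconds after each Movement Done event.
; On overlap with the player, it writes its actor location to PlayerPositionSpawn in GI_F4LGameInstance, then destroys itself.
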(event Collision|EventActorBeginOverlap
  (params (OtherActor :type Actor%20Object%20Reference))
  (Utilities|IsPlayer OtherActor
    (:IsPlayer
      (bind _asgi_f4lgame_instance (Utilities|Casting|CastToGI_F4LGameInstance (Game|GetGameInstance)))
      (Variables|/Game/GameInstances/GI_F4LGameInstance.GI_F4LGameInstance_C|SetplayerPositionSpawn _asgi_f4lgame_instance (Transformation|GetActorLocation))
      (Actor|DestroyActor))))

(event EventTick
  (params (DeltaSeconds :type Float%20%28single-precision%29)))

(event EventBeginPlay
  (bind _updownmovement (Timeline|upDownCheckpoint PlayFromStart)
    (:Update
      (Transformation|SetRelativeLocation (Variables|Default|GetBox) (Math|Vector|MakeVector 0.0 0.0 _updownmovement) false false))
    (:MovementDone
      (Utilities|FlowControl|Delay 2.0)
      (Timeline|upDownCheckpoint PlayFromStart))))

(fn ConstructionScript)