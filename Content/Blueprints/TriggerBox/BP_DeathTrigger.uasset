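; BP_DeathTrigger is a trigger volume that costs the player a life and leads to either respawn or game over.
; On BeginPlay it stores the first found PlayerStart's location in GI_F4LGameInstance as the spawn position.
; Box overlap starts a death camera fade on the other actor.
; The unfiltered actor overlap waits briefly, calls LoseLife, then branches via IsAlive to Respawn or GameOver.
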(event OnComponentBeginOverlap(Box)
  (params (OverlappedComponent :type Primitive%20Component%20Object%20Reference) (OtherActor :type Actor%20Object%20Reference) (OtherComp :type Primitive%20Component%20Object%20Reference) (OtherBodyIndex :type Integer) (bFromSweep :type Boolean) (SweepResult :type Hit%20Result%20Structure%20%28by%20ref%29))
  (Utilities|CameraFadeDeath OtherActor))

(event EventBeginPlay
  (Utilities|FlowControl|DoOnce false
    (:Completed
      (CallFunction|SetPlayerOriginalLocation))))

(event Collision|EventActorBeginOverlap
  (params (OtherActor :type Actor%20Object%20Reference))
  (Utilities|FlowControl|Delay 2.0)
  (bind _remaininglives (Utilities|LoseLife)
    (:.
      (Utilities|IsAlive _remaininglives
        (:Alive
          (Utilities|Respawn))
        (:Dead
          (Utilities|GameOver))))))

(event EventTick
  (params (DeltaSeconds :type Float%20%28single-precision%29)))

(fn ConstructionScript)

(fn SetPlayerOriginalLocation
  (bind _asf4lgame_instance (Utilities|Casting|CastToGI_F4LGameInstance (Game|GetGameInstance)))
  (bind _returnvalue (Actor|GetActorOfClass "/Script/Engine.PlayerStart"))
  (Variables|/Game/GameInstances/GI_F4LGameInstance.GI_F4LGameInstance_C|SetplayerPositionSpawn _asf4lgame_instance (Transformation|GetActorLocation _returnvalue)))