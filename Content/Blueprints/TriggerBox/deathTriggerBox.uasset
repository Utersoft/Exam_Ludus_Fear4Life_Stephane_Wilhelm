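; Death trigger volume that respawns the player at a PlayerStart and costs a life.
; Any actor overlap waits two seconds, moves the player pawn, then decrements Lives in F4LGameInstance.
; When lives run out, it reopens Fear4Life_Level1 and resets lives and grabbed collectibles.
; A separate Box overlap, filtered to the player pawn, fades the camera out to red and back in from green around the respawn delay.
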(event OnComponentBeginOverlap(Box)
  (params (OverlappedComponent :type Primitive%20Component%20Object%20Reference) (OtherActor :type Actor%20Object%20Reference) (OtherComp :type Primitive%20Component%20Object%20Reference) (OtherBodyIndex :type Integer) (bFromSweep :type Boolean) (SweepResult :type Hit%20Result%20Structure%20%28by%20ref%29))
  (if (== OtherActor (Game|Player|GetPlayerPawn 0))
    (CameraFades|StartCameraFade (Game|GetPlayerCameraManager 0) 0.0 1.0 2.0 "(R=1.000000,G=0.006983,B=0.000000,A=1.000000)" false false)
    (Utilities|FlowControl|Delay 2.0)
    (CameraFades|StartCameraFade (Game|GetPlayerCameraManager 0) 1.0 0.0 2.0 "(R=0.000000,G=1.000000,B=0.036782,A=1.000000)" false false)))

(event EventBeginPlay)

(event Collision|EventActorBeginOverlap
  (params (OtherActor :type Actor%20Object%20Reference))
  (Utilities|FlowControl|Delay 2.0)
  (bind _returnvalue (Actor|GetActorOfClass "/Script/Engine.PlayerStart"))
  (Transformation|SetRelativeLocation (Variables|/Script/Engine.Actor|GetRootComponent (Game|Player|GetPlayerPawn 0)) (Transformation|GetActorLocation _returnvalue) false false)
  (bind _asf4lgame_instance (Utilities|Casting|CastToF4LGameInstance (Game|GetGameInstance)))
  (bind _output_get (Variables|/Game/GameInstances/F4LGameInstance.F4LGameInstance_C|SetLives _asf4lgame_instance (- (Variables|/Game/GameInstances/F4LGameInstance.F4LGameInstance_C|GetLives _asf4lgame_instance) 1)))
  (if (<= _output_get 0)
    (Game|OpenLevel(byName) "Fear4Life_Level1")
    (bind _asf4lgame_instance_2 (Utilities|Casting|CastToF4LGameInstance (Game|GetGameInstance)))
    (Variables|/Game/GameInstances/F4LGameInstance.F4LGameInstance_C|SetgrabbedCollectibles _asf4lgame_instance_2 0)
    (Variables|/Game/GameInstances/F4LGameInstance.F4LGameInstance_C|SetLives _asf4lgame_instance_2 3)))

(event EventTick
  (params (DeltaSeconds :type Float%20%28single-precision%29)))

(fn ConstructionScript)