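; End-of-level trigger box that, when the player pawn overlaps it, opens the next level in LevelsNames or quits the game on the last.
; Level order comes from finding the current level name in that array.
; The last-level test compares array length to that index, which a found index never equals.
; After requesting the level load, it adds a GameInstance life if no F4L_Collectibles actors remain.
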(event EventBeginPlay)

(event Collision|EventActorBeginOverlap
  (params (OtherActor :type Actor%20Object%20Reference))
  (|IsPlayer OtherActor
    (:IsPlayer
      (if (CallFunction|IsLastLevel)
        (Game|QuitGame 0 "Quit" false)
        (else
          (Game|OpenLevel(byName) (CallFunction|GetNextLevelName))
          (bind _asf4l_collectibles (Utilities|Casting|CastToF4L_CollectiblesClass "/Game/Blueprints/Collectibles/F4L_Collectibles.F4L_Collectibles_C"))
          (bind _outactors (Actor|GetAllActorsOfClass _asf4l_collectibles))
          (if (<= (Utilities|Array|Length _outactors) 0)
            (bind _asf4lgame_instance (Utilities|Casting|CastToF4LGameInstance (Game|GetGameInstance)))
            (Variables|/Game/GameInstances/F4LGameInstance.F4LGameInstance_C|SetLives _asf4lgame_instance (+ (Variables|/Game/GameInstances/F4LGameInstance.F4LGameInstance_C|GetLives _asf4lgame_instance) 1))))))))

(event EventTick
  (params (DeltaSeconds :type Float%20%28single-precision%29)))

(fn ConstructionScript)

(fn GetLevelIndex
  (bind _returnvalue (Game|GetCurrentLevelName true))
  (return (Utilities|Array|FindItem (Variables|Default|GetLevelsNames) (Utilities|String|StringToName _returnvalue))))

(fn IsLastLevel
  (return (== (Utilities|Array|Length (Variables|Default|GetLevelsNames)) (CallFunction|GetLevelIndex))))

(fn GetNextLevelName
  (return (Utilities|Array|Get(acopy) (Variables|Default|GetLevelsNames) (+ (CallFunction|GetLevelIndex) 1))))